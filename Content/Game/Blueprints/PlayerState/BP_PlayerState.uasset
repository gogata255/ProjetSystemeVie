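; BP_PlayerState is the player state that mirrors the player's health into the game instance.
; On BeginPlay it caches a BP_GameInstance reference.
; Its AC_Health component's OnHealthChanged event writes current and max health to that instance through two save functions, so the values sit outside the player state.
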(event `self.ReceiveBeginPlay`
  (bind _asbp_game_instance (cast `/Game/Game/Blueprints/BP_GameInstance` (`GameplayStatics.GetGameInstance`)))
  (set `self.RefGameInstance` _asbp_game_instance))

(event `self.AC_Health.OnHealthChanged`
  (params (CurrentHealth :type "Float (double-precision)") (MaxHealth :type "Float (double-precision)"))
  (`self.SaveCurrentHealth` CurrentHealth)
  (`self.SaveMaxHealth` MaxHealth))

(fn `SaveCurrentHealth`
  (params (NewHealth :type "Float (double-precision)"))
  (set `/Game/Game/Blueprints/BP_GameInstance.CurrentHealth_GI` NewHealth (`self.RefGameInstance`)))

(fn `SaveMaxHealth`
  (params (NewMaxHealth :type "Float (double-precision)"))
  (set `/Game/Game/Blueprints/BP_GameInstance.MaxHealth_GI` NewMaxHealth (`self.RefGameInstance`)))

(fn `UserConstructionScript`)